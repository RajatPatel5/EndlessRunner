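; BP_Coins is a coin pickup that the ThirdPersonCharacter collects by touch and can attract with a magnet.
; Overlapping the Coin component destroys the actor and plays a pickup sound at the player's location.
; Overlapping MagnetSphere while the character's IsMagnetActive is set starts a timeline.
; Each update moves the coin with sweep toward the player using VInterpTo, adding the timeline track as an offset.
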(event `self.Coin.OnComponentBeginOverlap`
  (params (OverlappedComponent :type "PrimitiveComponent Object Reference") (OtherActor :type "Actor Object Reference") (OtherComp :type "PrimitiveComponent Object Reference") (OtherBodyIndex :type Integer) (bFromSweep :type Boolean) (SweepResult :type "HitResult Structure (by ref)"))
  (cast `/Game/ThirdPersonBP/Blueprints/ThirdPersonCharacter` OtherActor)
  (`self.K2_DestroyActor`)
  (`GameplayStatics.PlaySoundAtLocation` "/Game/Sounds/CoinsPickSound.CoinsPickSound" (`self.K2_GetActorLocation` (`GameplayStatics.GetPlayerCharacter` 0)) (struct) 1.0 1.0 0.0 null null null))

(event `self.MagnetSphere.OnComponentBeginOverlap`
  (params (OverlappedComponent :type "PrimitiveComponent Object Reference") (OtherActor :type "Actor Object Reference") (OtherComp :type "PrimitiveComponent Object Reference") (OtherBodyIndex :type Integer) (bFromSweep :type Boolean) (SweepResult :type "HitResult Structure (by ref)"))
  (bind _asthird_person_character (cast `/Game/ThirdPersonBP/Blueprints/ThirdPersonCharacter` OtherActor))
  (if (`/Game/ThirdPersonBP/Blueprints/ThirdPersonCharacter.isMagnetActive` _asthird_person_character)
    (bind (_direction _newtrack_1) (`Timeline|Timeline_0`)
      (:`Update`
        (`self.K2_SetActorLocation` (+ _newtrack_1 (`KismetMathLibrary.VInterpTo` (.location (`self.GetTransform`)) (`self.K2_GetActorLocation` (`GameplayStatics.GetPlayerCharacter` 0)) (`GameplayStatics.GetWorldDeltaSeconds`) 30.0)) true)))))

(fn `UserConstructionScript`)