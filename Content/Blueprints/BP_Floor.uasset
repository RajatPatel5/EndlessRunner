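; Floor tile for an endlessly extended track that asks the game mode to add floors when the player overlaps it, then destroys itself shortly after.
; The overlap increments the character's Counts until it exceeds two, then instead calls SpawnShields on a parent BP_SpawnPowerUps actor.
; The construction script adds coin child actors at randomly picked marker positions, which may repeat; obstacle spawning is disconnected.
; AddFloor returns the attach transform for the next tile.
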(event `self.Collision.OnComponentBeginOverlap`
  (params (OverlappedComponent :type "PrimitiveComponent Object Reference") (OtherActor :type "Actor Object Reference") (OtherComp :type "PrimitiveComponent Object Reference") (OtherBodyIndex :type Integer) (bFromSweep :type Boolean) (SweepResult :type "HitResult Structure (by ref)"))
  (bind _asthird_person_character (cast `/Game/ThirdPersonBP/Blueprints/ThirdPersonCharacter` OtherActor))
  (bind _asthird_person_game_mode (cast `/Game/ThirdPersonBP/Blueprints/ThirdPersonGameMode` (`GameplayStatics.GetGameMode`)))
  (`/Game/ThirdPersonBP/Blueprints/ThirdPersonGameMode.AddFloorsInGame` _asthird_person_game_mode)
  (bind _counts (`/Game/ThirdPersonBP/Blueprints/ThirdPersonCharacter.Counts` _asthird_person_character))
  (`KismetSystemLibrary.PrintString` (`KismetStringLibrary.Conv_IntToString` _counts))
  (if (> _counts 2)
    (bind _asbp_spawn_power_ups (cast `/Game/Blueprints/BP_SpawnPowerUps` (`self.GetParentActor`)))
    (`/Game/Blueprints/BP_SpawnPowerUps.SpawnShields` _asbp_spawn_power_ups)
    (else
      (set `/Game/ThirdPersonBP/Blueprints/ThirdPersonCharacter.Counts` (+ _counts 1) _asthird_person_character)))
  (`KismetSystemLibrary.Delay` 2.0)
  (`self.K2_DestroyActor`))

(fn `AddFloor`
  (returns (NewParam :type "Transform Structure"))
  (return (`SceneComponent.K2_GetComponentToWorld` (`self.SpawnNextFloorPointer`))))

(fn `CoinsSpawnPositions`
  (set `self.CoinSpawnPositions` (`|MakeArray` (`SceneComponent.GetRelativeTransform` (`self.CoinSpawn`)) (`SceneComponent.GetRelativeTransform` (`self.CoinSpawn1`)) (`SceneComponent.GetRelativeTransform` (`self.CoinSpawn2`)) (`SceneComponent.GetRelativeTransform` (`self.CoinSpawn3`)))))

(fn `ObstacleSpawnPositions`)

(fn `SpawnCoins`
  (bind _coinspawnpositions (`self.CoinSpawnPositions`))
  (for _ (range 4)
    (`AddComponent|NODE_AddChildActorComponent-1` :`RelativeTransform` (`|GetArrayItem` _coinspawnpositions (`KismetMathLibrary.RandomIntegerInRange` 0 (`KismetArrayLibrary.Array_LastIndex` _coinspawnpositions))))))

(fn `SpawnObstacles`
  ;[1 1 1] Comment
)

(fn `UserConstructionScript`
  (`self.CoinsSpawnPositions`)
  (`self.SpawnCoins`))