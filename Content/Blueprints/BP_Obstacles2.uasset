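; BP_Obstacles2 is an obstacle actor that ends the run when the ThirdPersonCharacter hits its Cube component.
; An active shield absorbs the hit: the obstacle destroys itself, hides the character's Sphere and clears IsShieldActive.
; Otherwise it destroys the player character, switches to UI-only input with a visible cursor, and replaces all widgets with LoseScreen_HUD.
; An unconnected copy of the lose sequence remains in the event graph and never runs.
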(event `self.Cube.OnComponentHit`
  (params (HitComponent :type "PrimitiveComponent Object Reference") (OtherActor :type "Actor Object Reference") (OtherComp :type "PrimitiveComponent Object Reference") (NormalImpulse :type "Vector Structure") (Hit :type "HitResult Structure (by ref)"))
  (bind _returnvalue (`GameplayStatics.GetPlayerController` 0))
  (bind _asthird_person_character (cast `/Game/ThirdPersonBP/Blueprints/ThirdPersonCharacter` OtherActor))
  (if (`/Game/ThirdPersonBP/Blueprints/ThirdPersonCharacter.IsShieldActive` _asthird_person_character)
    (`self.K2_DestroyActor`)
    (`SceneComponent.SetVisibility` (`/Game/ThirdPersonBP/Blueprints/ThirdPersonCharacter.Sphere` _asthird_person_character) false false)
    (set `/Game/ThirdPersonBP/Blueprints/ThirdPersonCharacter.IsShieldActive` false _asthird_person_character)
    (else
      (`self.DisableInput` _returnvalue)
      (`self.K2_DestroyActor` (`GameplayStatics.GetPlayerCharacter` 0))
      (`WidgetBlueprintLibrary.SetInputMode_UIOnlyEx` _returnvalue null)
      (`WidgetLayoutLibrary.RemoveAllWidgets`)
      (bind _returnvalue_2 (`|CreateWidget` "/Game/UI/LoseScreen_HUD.LoseScreen_HUD_C"))
      (`UserWidget.AddToViewport` _returnvalue_2 0)
      (set `PlayerController.bShowMouseCursor` true _returnvalue))))

(fn `UserConstructionScript`)